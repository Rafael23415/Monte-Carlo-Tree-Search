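; Tic-tac-toe game Blueprint that pits a human against a machine, with a nine-cell board state.
; Number keys 1–9 place the human's move, then pass the current state to the Tree's NextTurn.
; CreateCells spawns a BP_Cell at each of nine scene components.
; CheckWin runs the CheckLine macro over all eight lines to report the winning side, a full-board draw or an unfinished game.
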(event `Key|One`
  (params (Key :type "Key Structure"))
  (:`Pressed`
    (`self.MakeMove` "NewEnumerator1")
    (`/Game/MCTS/BP_Tree.NextTurn` (`self.Tree`) (`self.GetCurrentState`) :!label _label)))

(event `Key|Two`
  (params (Key :type "Key Structure"))
  (:`Pressed`
    (`self.MakeMove` "NewEnumerator1" 1)
    (goto _label)))

(event `Key|Three`
  (params (Key :type "Key Structure"))
  (:`Pressed`
    (`self.MakeMove` "NewEnumerator1" 2)
    (goto _label)))

(event `Key|Four`
  (params (Key :type "Key Structure"))
  (:`Pressed`
    (`self.MakeMove` "NewEnumerator1" 3)
    (goto _label)))

(event `Key|Five`
  (params (Key :type "Key Structure"))
  (:`Pressed`
    (`self.MakeMove` "NewEnumerator1" 4)
    (goto _label)))

(event `Key|Six`
  (params (Key :type "Key Structure"))
  (:`Pressed`
    (`self.MakeMove` "NewEnumerator1" 5)
    (goto _label)))

(event `Key|Seven`
  (params (Key :type "Key Structure"))
  (:`Pressed`
    (`self.MakeMove` "NewEnumerator1" 6)
    (goto _label)))

(event `Key|Eight`
  (params (Key :type "Key Structure"))
  (:`Pressed`
    (`self.MakeMove` "NewEnumerator1" 7)
    (goto _label)))

(event `Key|Nine`
  (params (Key :type "Key Structure"))
  (:`Pressed`
    (`self.MakeMove` "NewEnumerator1" 8)
    (goto _label)))

(fn `CheckWin`
  (params (State :type "Array of /Game/MCTS/E_CellType Enum (by ref)" :default _))
  (returns (WonSide :type "/Game/MCTS/E_WinState Enum"))
  (locals (Win :type "/Game/MCTS/E_WinState Enum"))
  (bind (_bresult _win) (`self.CheckLine` State 0 1 2)
    (:`Won`
      (set `local.Win` _win))
    (:`Nothing`
      (bind (_bresult_2 _win_2) (`self.CheckLine` State 3 4 5)
        (:`Won`
          (set `local.Win` _win_2))
        (:`Nothing`
          (bind (_bresult_3 _win_3) (`self.CheckLine` State 6 7 8)
            (:`Won`
              (set `local.Win` _win_3))
            (:`Nothing`
              (bind (_bresult_4 _win_4) (`self.CheckLine` State 0 3 6)
                (:`Won`
                  (set `local.Win` _win_4))
                (:`Nothing`
                  (bind (_bresult_5 _win_5) (`self.CheckLine` State 1 4 7)
                    (:`Won`
                      (set `local.Win` _win_5))
                    (:`Nothing`
                      (bind (_bresult_6 _win_6) (`self.CheckLine` State 2 5 8)
                        (:`Won`
                          (set `local.Win` _win_6))
                        (:`Nothing`
                          (bind (_bresult_7 _win_7) (`self.CheckLine` State 0 4 8)
                            (:`Won`
                              (set `local.Win` _win_7))
                            (:`Nothing`
                              (bind (_bresult_8 _win_8) (`self.CheckLine` State 2 4 6)
                                (:`Won`
                                  (set `local.Win` _win_8))
                                (:`Nothing`
                                  (set `local.Win` "NewEnumerator0")))))))))))))))))
  (if (or _bresult _bresult_2 _bresult_3 _bresult_4 _bresult_5 _bresult_6 _bresult_7 _bresult_8)
    _
    (elif (== (`KismetArrayLibrary.Array_Find` State "NewEnumerator0") -1)
      (set `local.Win` "NewEnumerator2")
      (else
        (set `local.Win` "NewEnumerator0"))))
  (return (`local.Win`)))

(fn `CreateCells`
  (for _index (range 9)
    (bind _returnvalue (`|SpawnActorFromClass` "/Game/MCTS/BP_Cell.BP_Cell_C" (`KismetMathLibrary.MakeTransform` (`SceneComponent.K2_GetComponentLocation` (select `int` _index :`0` (`self.Scene`) :`1` (`self.Scene1`) :`2` (`self.Scene2`) :`3` (`self.Scene3`) :`4` (`self.Scene4`) :`5` (`self.Scene5`) :`6` (`self.Scene6`) :`7` (`self.Scene7`) :`8` (`self.Scene8`)))) "Undefined" "MultiplyWithRoot" null null))
    (`KismetArrayLibrary.Array_Add` (`self.Cells`) _returnvalue)))

(fn `UserConstructionScript`
  (set `self.StateSize` 9))