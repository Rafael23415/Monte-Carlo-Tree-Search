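; A Monte Carlo Tree Search node for a turn-based Human-versus-Machine board game, holding a board state, visits and value.
; Expand moves a random pending child into the active children and simulates it.
; Simulate pre-generates that node's child states through the Tree, then plays random alternating moves until CheckWin returns a result.
; Backpropagation recursively scores each ancestor from its CurrentPlayer's perspective, then sets a short timer at the root.
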(fn `Backpropagation`
  (params (WhoWon :type "/Game/MCTS/E_WinState Enum" :default "NewEnumerator0"))
  (bind _currentplayer (`self.CurrentPlayer`))
  (`KismetSystemLibrary.PrintString` (`self.Tree`) "Backpropagation")
  (set `self.Value` (+ (`self.Value`) (select `/Game/MCTS/E_WinState` WhoWon :`NewEnumerator1` (select `/Game/MCTS/E_CellType` _currentplayer :`NewEnumerator1` 1 :`NewEnumerator2` -1) :`NewEnumerator3` (select `/Game/MCTS/E_CellType` _currentplayer :`NewEnumerator1` -1 :`NewEnumerator2` 1))))
  (`/Engine/EditorBlueprintResources/StandardMacros.IncrementInt` (`self.Visits`)
    (:`  `
      (`self.Print`)
      (if (!= self (`/Game/MCTS/BP_Tree.RootNode` (`self.Tree`)))
        (`self.Backpropagation` (`self.ParentNode`) WhoWon)
        (else
          (`KismetSystemLibrary.K2_SetTimerDelegate` (`|CreateDelegate` (`self.Tree`) :!event `FinishedBackPropagation`) 0.0001))))))

(fn `CreatePossibleStates`
  (locals (TemporaryState :type "Array of /Game/MCTS/E_CellType Enum"))
  (if (not (`self.bIsTerminal`))
    (for (_array_element _array_index) (`self.State`)
      (if (`|EnumEquality` _array_element "NewEnumerator0")
        (bind _output_get (set `local.TemporaryState` (`self.State`)))
        (`KismetArrayLibrary.Array_Set` _output_get _array_index (`self.CurrentPlayer`))
        (bind _wonside (`/Game/MCTS/BP_Tree.CheckWin` (`self.Tree`) (`local.TemporaryState`)))
        (`/Game/MCTS/BP_Tree.CreateNode` (`self.Tree`) self (`local.TemporaryState`) (`|EnumInequality` _wonside "NewEnumerator0"))))
    (`KismetSystemLibrary.PrintString` (`self.Tree`) (`KismetStringLibrary.Concat_StrStr` "Created all states for node " (`self.Name`)))
    (set `self.bIsFullyExpanded` (== (`KismetArrayLibrary.Array_Length` (`self.RemainingPossibleNodes`)) 0))))

(fn `Expand`
  (locals (SelectedChild :type "/Game/MCTS/BP_Node Object Reference"))
  (bind _output_get (set `local.SelectedChild` (`|GetArrayItem` (`self.RemainingPossibleNodes`) (`KismetMathLibrary.RandomInteger` (`KismetArrayLibrary.Array_Length` (`self.RemainingPossibleNodes`))))))
  (`KismetSystemLibrary.PrintString` (`self.Tree`) (`KismetStringLibrary.Concat_StrStr` "Expanding to " (`/Game/MCTS/BP_Node.Name` _output_get)))
  (bind _selectedchild (`local.SelectedChild`)
    (:`then`
      (`KismetArrayLibrary.Array_Add` (`self.ChildrenNodes`) _selectedchild)
      (`KismetArrayLibrary.Array_RemoveItem` (`self.RemainingPossibleNodes`) _selectedchild)
      (if (not (> (`KismetArrayLibrary.Array_Length` (`self.RemainingPossibleNodes`)) 0))
        (set `self.bIsFullyExpanded` true))
      (`self.Simulate` (`local.SelectedChild`)))
    (:`else`)))

(fn `Print`
  (bind _parentnode (`self.ParentNode`))
  (`KismetSystemLibrary.PrintString` (`self.Tree`) (`KismetStringLibrary.Concat_StrStr` "Name: " (`self.Name`) " | Parent Name: " (select `bool` (`KismetSystemLibrary.IsValid` _parentnode) :`false` "Root" :`true` (`/Game/MCTS/BP_Node.Name` _parentnode)) " | Number Of Active Children: " (`KismetStringLibrary.Conv_IntToString` (`KismetArrayLibrary.Array_Length` (`self.ChildrenNodes`))) " | Number Of Inactive Children: " (`KismetStringLibrary.Conv_IntToString` (`KismetArrayLibrary.Array_Length` (`self.RemainingPossibleNodes`))) " | Value: " (`KismetStringLibrary.Conv_IntToString` (`self.Value`)) " | Visits: " (`KismetStringLibrary.Conv_IntToString` (`self.Visits`)) " | Fully Expanded: " (`KismetStringLibrary.Conv_BoolToString` (`self.bIsFullyExpanded`)) " | Terminal: " (`KismetStringLibrary.Conv_BoolToString` (`self.bIsTerminal`)) " | Who is playing: " (`|GetEnumeratorNameAsString` (`self.CurrentPlayer`)))))

(fn `PrintState`
  (params (State :type "Array of /Game/MCTS/E_CellType Enum"))
  (for _array_element State
    (`KismetSystemLibrary.PrintString` (`self.Tree`) (`|GetEnumeratorNameAsString` _array_element)))
  (return))

(fn `Simulate`
  (locals (RandomIndex :type Integer) (CurrentWin :type "/Game/MCTS/E_WinState Enum") (TemporaryState :type "Array of /Game/MCTS/E_CellType Enum"))
  (bind _temporarystate (`local.TemporaryState`))
  (bind _temporarystate_2 (`local.TemporaryState`))
  (set `local.CurrentWin` "NewEnumerator0")
  (`self.CreatePossibleStates`)
  (set `local.TemporaryState` (`self.State`))
  (`KismetSystemLibrary.PrintString` (`self.Tree`) (`KismetStringLibrary.Concat_StrStr` "Simulating " (`self.Name`)))
  (`KismetSystemLibrary.PrintString` (`self.Tree`) "Current state:")
  (`self.PrintState` (`self.State`))
  (if (`|EnumEquality` (`local.CurrentWin`) "NewEnumerator0") :!label _label
    (set `local.RandomIndex` (`KismetMathLibrary.RandomInteger` (`KismetArrayLibrary.Array_Length` _temporarystate)))
    (bind _wonside (`/Game/MCTS/BP_Tree.CheckWin` (`self.Tree`) (`local.TemporaryState`)))
    (bind _output_get (set `local.CurrentWin` _wonside))
    (if (`|EnumEquality` (`|GetArrayItem` _temporarystate (`local.RandomIndex`)) "NewEnumerator0")
      (if (`|EnumEquality` _output_get "NewEnumerator0")
        (`/Engine/EditorBlueprintResources/StandardMacros.FlipFlop`
          (:`A`
            (`KismetArrayLibrary.Array_Set` _temporarystate_2 (`local.RandomIndex`) (`self.CurrentPlayer`))
            (goto _label))
          (:`B`
            (`KismetArrayLibrary.Array_Set` _temporarystate_2 (`local.RandomIndex`) (`/Game/MCTS/BP_Node.CurrentPlayer` (`self.ParentNode`)))
            (goto _label)))
        (else
          (goto _label)))
      (else
        (goto _label)))
    (else
      (`KismetSystemLibrary.PrintString` (`self.Tree`) "Simulated state:")
      (`self.PrintState` (`local.TemporaryState`))
      (`KismetSystemLibrary.PrintString` (`self.Tree`) (select `/Game/MCTS/E_WinState` (`local.CurrentWin`) :`NewEnumerator0` "Error" :`NewEnumerator1` "Lose" :`NewEnumerator2` "Draw" :`NewEnumerator3` "Win"))
      (`self.Backpropagation` (`local.CurrentWin`)))))