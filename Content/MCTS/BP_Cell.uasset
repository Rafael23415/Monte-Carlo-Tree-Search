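; BP_Cell is a game cell actor in the MCTS folder that shows whether it is empty or held by the human or the machine.
; SetType stores the new state in CurrentType and toggles two cylinder components, so Human and Machine each show their own marker and Nothing hides both.
; The cell resets to Nothing on BeginPlay, and every SetType call prints the current and incoming state for debugging.
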(event `self.ReceiveBeginPlay`
  (`self.SetType` "NewEnumerator0"))

(fn `SetType`
  (params (NewType :type "/Game/MCTS/E_CellType Enum" :default "NewEnumerator0"))
  (bind _cylinder (`self.Cylinder`))
  (`KismetSystemLibrary.PrintString` (`KismetStringLibrary.Concat_StrStr` (`KismetSystemLibrary.GetDisplayName` self) " current type " (`|GetEnumeratorNameAsString` (`self.CurrentType`)) " getting type " (`|GetEnumeratorNameAsString` NewType)))
  (bind _output_get (set `self.CurrentType` NewType))
  (switch `/Game/MCTS/E_CellType` _output_get
    (:`NewEnumerator0`
      (`SceneComponent.SetHiddenInGame` _cylinder true false)
      (`SceneComponent.SetHiddenInGame` (`self.Cylinder1`) true false))
    (:`NewEnumerator1`
      (`SceneComponent.SetHiddenInGame` (`self.Cylinder1`) false false)
      (`SceneComponent.SetHiddenInGame` (`self.Cylinder`) true false))
    (:`NewEnumerator2`
      (`SceneComponent.SetHiddenInGame` _cylinder false false)
      (`SceneComponent.SetHiddenInGame` (`self.Cylinder1`) true false))))

(fn `UserConstructionScript`)