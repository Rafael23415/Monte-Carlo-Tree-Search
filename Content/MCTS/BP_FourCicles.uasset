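; BP_FourCicles is a four-cell, one-row board game between a human and a machine, built on an MCTS tree.
; Keys 1–4 place the human's move, then pass the current state to the tree for the next turn.
; CreateCells spawns a BP_Cell at four scene component locations.
; CheckWin awards a win for two adjacent matching marks and flags a separate result for a full board without one.
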(event `Key|One`
  (params (Key :type "Key Structure"))
  (:`Pressed`
    (`self.MakeMove` "NewEnumerator1")
    (`/Game/MCTS/BP_Tree.NextTurn` (`self.Tree`) (`self.GetCurrentState`) :!label _label)))

(event `Key|Two`
  (params (Key :type "Key Structure"))
  (:`Pressed`
    (`self.MakeMove` "NewEnumerator1" 1)
    (goto _label)))

(event `Key|Three`
  (params (Key :type "Key Structure"))
  (:`Pressed`
    (`self.MakeMove` "NewEnumerator1" 2)
    (goto _label)))

(event `Key|Four`
  (params (Key :type "Key Structure"))
  (:`Pressed`
    (`self.MakeMove` "NewEnumerator1" 3)
    (goto _label)))

(fn `CheckWin`
  (params (State :type "Array of /Game/MCTS/E_CellType Enum (by ref)" :default _))
  (returns (WonSide :type "/Game/MCTS/E_WinState Enum"))
  (locals (Win :type "/Game/MCTS/E_WinState Enum"))
  (set `local.Win` "NewEnumerator0")
  (for (_array_element _array_index) State
    (if (!= _array_index (- (`KismetArrayLibrary.Array_Length` State) 1))
      (bind _output (`|GetArrayItem` State (+ _array_index 1)))
      (if (and (`|EnumEquality` _array_element _output) (`|EnumInequality` _output "NewEnumerator0") (`|EnumInequality` _array_element "NewEnumerator0"))
        (set `local.Win` (select `/Game/MCTS/E_CellType` _output :`NewEnumerator0` "NewEnumerator0" :`NewEnumerator1` "NewEnumerator1" :`NewEnumerator2` "NewEnumerator3" :!type "/Game/MCTS/E_WinState Enum"))
        (break))
      (else
        (break))))
  (if (and (== (`KismetArrayLibrary.Array_Find` State "NewEnumerator0") -1) (`|EnumEquality` (`local.Win`) "NewEnumerator0"))
    (set `local.Win` "NewEnumerator2"))
  (return (`local.Win`)))

(fn `CreateCells`
  (for _index (range 4)
    (bind _returnvalue (`|SpawnActorFromClass` "/Game/MCTS/BP_Cell.BP_Cell_C" (`KismetMathLibrary.MakeTransform` (`SceneComponent.K2_GetComponentLocation` (select `int` _index :`0` (`self.Scene`) :`1` (`self.Scene1`) :`2` (`self.Scene2`) :`3` (`self.Scene3`)))) "Undefined" "MultiplyWithRoot" null null))
    (`KismetArrayLibrary.Array_Add` (`self.Cells`) _returnvalue)))

(fn `UserConstructionScript`
  (set `self.StateSize` 4))