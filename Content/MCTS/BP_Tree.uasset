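; Monte Carlo Tree Search manager that picks the Machine's moves against a Human on a Board.
; Selection descends BP_Node children by UCT with negated values for alternating players, then expands or simulates.
; FinishedBackPropagation repeats selection up to MaxIterations, then MakeMove applies the most-visited child to the Board and re-roots there.
; NextTurn matches the received state to an expanded or pending child, reusing that subtree for the next search.
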(event EventBeginPlay
  (Default|Start (Variables|Default|GetBoard))
  (bind _returnvalue (Game|ConstructObjectfromClass "/Game/MCTS/BP_Node.BP_Node_C"))
  (Variables|Default|SetRootNode _returnvalue)
  (Variables|/Game/MCTS/BP_Node.BP_Node_C|SetTree (Variables|Default|GetRootNode) self)
  (Variables|/Game/MCTS/BP_Node.BP_Node_C|SetName (Variables|Default|GetRootNode) "R")
  (Variables|/Game/MCTS/BP_Node.BP_Node_C|SetCurrentPlayer (Variables|Default|GetRootNode) "NewEnumerator2")
  (for _index (range 0 (- (Variables|/Game/MCTS/BP_Board.BP_Board_C|GetStateSize (Variables|Default|GetBoard)) 1))
    (Utilities|Array|Add (Variables|/Game/MCTS/BP_Node.BP_Node_C|GetState (Variables|Default|GetRootNode)) "NewEnumerator0"))
  (Default|CreatePossibleStates (Variables|Default|GetRootNode))
  (CallFunction|Selection (Variables|Default|GetRootNode)))

(fn ConstructionScript)

(fn Selection
  (params (RootNode :type BP%20Node%20Object%20Reference))
  (bind _output_get (Variables|Default|SetCurrentRootNode RootNode))
  ;[0.15 0.15 0.15 0.5] Check if doesn't have children yet, so expand right away
  (if (> (Utilities|Array|Length (Variables|/Game/MCTS/BP_Node.BP_Node_C|GetChildrenNodes _output_get)) 0)
    (if (not (Variables|/Game/MCTS/BP_Node.BP_Node_C|GetbIsFullyExpanded (Variables|Default|GetCurrentRootNode)))
      (Default|Expand (Variables|Default|GetCurrentRootNode))
      (else
        (LocalVariables|SetCurrentSelectedNode (Utilities|Array|Get(acopy) (Variables|/Game/MCTS/BP_Node.BP_Node_C|GetChildrenNodes _output_get)))
        (for _array_element (Variables|/Game/MCTS/BP_Node.BP_Node_C|GetChildrenNodes _output_get)
          (bind _uct (CallFunction|CalculateUCT _array_element))
          (bind _uct_2 (CallFunction|CalculateUCT (LocalVariables|GetCurrentSelectedNode)))
          (if (> _uct _uct_2)
            (LocalVariables|SetCurrentSelectedNode _array_element)))
        (Development|PrintString (Utilities|String|Append "Selected " (Variables|/Game/MCTS/BP_Node.BP_Node_C|GetName (LocalVariables|GetCurrentSelectedNode)) " with a UCT of " (Utilities|String|ToString(Float) _uct)))
        (if (not (Variables|/Game/MCTS/BP_Node.BP_Node_C|GetbIsTerminal (LocalVariables|GetCurrentSelectedNode)))
          (if (Variables|/Game/MCTS/BP_Node.BP_Node_C|GetbIsFullyExpanded (LocalVariables|GetCurrentSelectedNode))
            (CallFunction|Selection (LocalVariables|GetCurrentSelectedNode))
            (else
              (Default|Expand (LocalVariables|GetCurrentSelectedNode))))
          (else
            (Default|Simulate (LocalVariables|GetCurrentSelectedNode))))))
    (else
      (Default|Expand (Variables|Default|GetCurrentRootNode)))))

(fn CreateNode
  (params (ParentNode :type BP%20Node%20Object%20Reference) (State :type Array%20of%20E_CellType%20Enums :default "NewEnumerator0") (bIsTerminal :type Boolean))
  (bind _remainingpossiblenodes (Variables|/Game/MCTS/BP_Node.BP_Node_C|GetRemainingPossibleNodes ParentNode))
  (bind _returnvalue (Game|ConstructObjectfromClass "/Game/MCTS/BP_Node.BP_Node_C"))
  (Utilities|Array|Add _remainingpossiblenodes _returnvalue)
  (Variables|/Game/MCTS/BP_Node.BP_Node_C|SetParentNode _returnvalue ParentNode)
  (Variables|/Game/MCTS/BP_Node.BP_Node_C|SetState _returnvalue State)
  (Variables|/Game/MCTS/BP_Node.BP_Node_C|SetCurrentPlayer _returnvalue (Utilities|Select :Index (Variables|/Game/MCTS/BP_Node.BP_Node_C|GetCurrentPlayer ParentNode) :NewEnumerator0 "NewEnumerator0" :NewEnumerator1 "NewEnumerator2" :NewEnumerator2 "NewEnumerator1"))
  (Variables|/Game/MCTS/BP_Node.BP_Node_C|SetTree _returnvalue self)
  (Variables|/Game/MCTS/BP_Node.BP_Node_C|SetbIsTerminal _returnvalue bIsTerminal)
  (Variables|/Game/MCTS/BP_Node.BP_Node_C|SetbIsFullyExpanded _returnvalue bIsTerminal)
  (Variables|/Game/MCTS/BP_Node.BP_Node_C|SetName _returnvalue (Utilities|String|Append (Variables|/Game/MCTS/BP_Node.BP_Node_C|GetName ParentNode) (Utilities|Select :Index (Utilities|Array|Length _remainingpossiblenodes) :Option%200 "" :Option%201 "A" :Option%202 "B" :Option%203 "C" :Option%204 "D" :Option%205 "E" :Option%206 "F" :Option%207 "G" :Option%208 "H" :Option%209 "I" :Option%2010 "J" :Option%2011 "K" :Option%2012 "L" :Option%2013 "M")))
  (Development|PrintString (Utilities|String|Append "Created " (Variables|/Game/MCTS/BP_Node.BP_Node_C|GetName _returnvalue)))
  (Default|Print _returnvalue)
  (return))

(fn CheckWin
  (params (State :type Array%20of%20E_CellType%20Enums :default "NewEnumerator0"))
  (bind _wonside (Default|CheckWin (Variables|Default|GetBoard) State))
  (return _wonside))

(fn FinishedBackPropagation
  (bind _iterations (Variables|Default|GetIterations))
  (Math|Integer|IncrementInt _iterations
    (:%20%20
      (if (< _iterations (Variables|Default|GetMaxIterations))
        (Development|PrintString "=======================================================================")
        (Development|PrintString "")
        (Development|PrintString "")
        (Development|PrintString "")
        (Development|PrintString "=======================================================================")
        (CallFunction|Selection (Variables|Default|GetRootNode))
        (else
          (Development|PrintString "=======================================================================")
          (Development|PrintString "")
          (Development|PrintString "")
          (Development|PrintString "")
          (Development|PrintString "FinishedIterating")
          (CallFunction|PrintNodes (Variables|Default|GetRootNode))
          (CallFunction|MakeMove))))))

(fn PrintNodes
  (params (Target :type BP%20Node%20Object%20Reference))
  (Default|Print Target)
  (if (not (Variables|/Game/MCTS/BP_Node.BP_Node_C|GetbIsTerminal Target))
    (for _array_element (Variables|/Game/MCTS/BP_Node.BP_Node_C|GetChildrenNodes Target)
      (CallFunction|PrintNodes _array_element))))

(fn MakeMove
  (LocalVariables|SetBestState (Utilities|Array|Get(acopy) (Variables|/Game/MCTS/BP_Node.BP_Node_C|GetChildrenNodes (Variables|Default|GetRootNode))))
  (for _array_element (Variables|/Game/MCTS/BP_Node.BP_Node_C|GetChildrenNodes (Variables|Default|GetRootNode))
    (if (< (Variables|/Game/MCTS/BP_Node.BP_Node_C|GetVisits (LocalVariables|GetBestState)) (Variables|/Game/MCTS/BP_Node.BP_Node_C|GetVisits _array_element))
      (LocalVariables|SetBestState _array_element)))
  (Development|PrintString (Utilities|String|Append "Selected " (Variables|/Game/MCTS/BP_Node.BP_Node_C|GetName (LocalVariables|GetBestState))))
  (Variables|Default|SetRootNode (LocalVariables|GetBestState))
  (for (_array_element_2 _array_index) (Variables|/Game/MCTS/BP_Node.BP_Node_C|GetState (LocalVariables|GetBestState))
    (if (Utilities|Enum|NotEqual(Enum) _array_element_2 "NewEnumerator0")
      (Default|MakeMove (Variables|Default|GetBoard) _array_element_2 _array_index))))

(fn CalculateUCT
  (params (Node :type BP%20Node%20Object%20Reference))
  (bind _visits (Variables|/Game/MCTS/BP_Node.BP_Node_C|GetVisits Node))
  (bind _parentnode (Variables|/Game/MCTS/BP_Node.BP_Node_C|GetParentNode Node))
  (bind _rootnode (Variables|Default|GetRootNode))
  (bind _returnvalue (Utilities|IsValid _parentnode))
  (bind _returnvalue_2 (select _returnvalue _parentnode _rootnode))
  (bind _visits_2 (Variables|/Game/MCTS/BP_Node.BP_Node_C|GetVisits _returnvalue_2))
  (return (Math|Float|SelectFloat (|((value/visits)+(c*(sqrt(((loge(rootVisits))/visits))))) (Math|Conversions|ToFloat(Integer) (* (Variables|/Game/MCTS/BP_Node.BP_Node_C|GetValue Node) -1)) _visits (Math|Float|Sqrt 2.0) _visits_2) 0.0 (and (!= _visits_2 0) (!= _visits 0)))))

(fn NextTurn
  (params (State :type Array%20of%20E_CellType%20Enums :default "NewEnumerator0"))
  (LocalVariables|SetReceivedState State)
  (bind _array_element (Utilities|Array|ForEachLoopwithBreak (Variables|/Game/MCTS/BP_Node.BP_Node_C|GetChildrenNodes (Variables|Default|GetRootNode)) :!label _label)
    (:LoopBody
      (bind _output_get (LocalVariables|SetCurrentCheckingNode _array_element))
      (bind _bisthesame (Utilities|SameState (Variables|/Game/MCTS/BP_Node.BP_Node_C|GetState _output_get) (LocalVariables|GetReceivedState)))
      (bind _output_get_2 (LocalVariables|SetbFoundNode _bisthesame))
      (if _output_get_2
        (goto _label Break)))
    (:Completed
      (if (LocalVariables|GetbFoundNode)
        (if (not (Variables|/Game/MCTS/BP_Node.BP_Node_C|GetbIsTerminal (LocalVariables|GetCurrentCheckingNode)))
          (Variables|Default|SetRootNode (LocalVariables|GetCurrentCheckingNode))
          (Variables|Default|SetIterations 0)
          (CallFunction|Selection (Variables|Default|GetRootNode))
          (else
            (Development|PrintString "End")))
        (else
          (Development|PrintString (Utilities|String|Append "Didn't find state in already expanded nodes in " (Variables|/Game/MCTS/BP_Node.BP_Node_C|GetName (Variables|Default|GetRootNode))))
          (bind _array_element_2 (Utilities|Array|ForEachLoopwithBreak (Variables|/Game/MCTS/BP_Node.BP_Node_C|GetRemainingPossibleNodes (Variables|Default|GetRootNode)) :!label _label_2)
            (:LoopBody
              (bind _output_get_3 (LocalVariables|SetCurrentCheckingNode _array_element_2))
              (bind _bisthesame_2 (Utilities|SameState (Variables|/Game/MCTS/BP_Node.BP_Node_C|GetState _output_get_3) (LocalVariables|GetReceivedState)))
              (bind _output_get_4 (LocalVariables|SetbFoundNode _bisthesame_2))
              (if _output_get_4
                (goto _label_2 Break)))
            (:Completed
              (if (LocalVariables|GetbFoundNode)
                (if (not (Variables|/Game/MCTS/BP_Node.BP_Node_C|GetbIsTerminal (LocalVariables|GetCurrentCheckingNode)))
                  (Utilities|Array|Add (Variables|/Game/MCTS/BP_Node.BP_Node_C|GetChildrenNodes (Variables|Default|GetRootNode)) (LocalVariables|GetCurrentCheckingNode))
                  (Utilities|Array|RemoveItem (Variables|/Game/MCTS/BP_Node.BP_Node_C|GetRemainingPossibleNodes (Variables|Default|GetRootNode)) (LocalVariables|GetCurrentCheckingNode))
                  (Development|PrintString (Utilities|String|Append "Selected " (Variables|/Game/MCTS/BP_Node.BP_Node_C|GetName (LocalVariables|GetCurrentCheckingNode))))
                  (Variables|Default|SetRootNode (LocalVariables|GetCurrentCheckingNode))
                  (Default|CreatePossibleStates (Variables|Default|GetRootNode))
                  (Variables|Default|SetIterations 0)
                  (CallFunction|Selection (Variables|Default|GetRootNode))
                  (else
                    (Development|PrintString "End")))
                (else
                  (Development|PrintString "Didn't find current state" true true "(R=1.000000,G=0.000000,B=0.000000,A=1.000000)"))))))))))