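; BP_Board is a game board for the MCTS setup, with stub CreateCells and CheckWin functions, likely meant for child boards.
; Start enables player input and builds cells; MakeMove validates and sets a cell, resetting the board on a win or full board.
; GetCurrentState flattens cell types into an array for win checks.
; It caches BP_Tree on BeginPlay, but the Tree's NextTurn call is disconnected.
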(event `self.ReceiveBeginPlay`
  (bind _returnvalue (`GameplayStatics.GetActorOfClass` "/Game/MCTS/BP_Tree.BP_Tree_C"))
  (set `self.Tree` _returnvalue))

(fn `CheckWin`
  (params (State :type "Array of /Game/MCTS/E_CellType Enum"))
  (returns (WonSide :type "/Game/MCTS/E_WinState Enum"))
  (return "NewEnumerator0"))

(fn `CreateCells`
  (return))

(fn `GetCurrentState`
  (returns (CurrentState :type "Array of /Game/MCTS/E_CellType Enum"))
  (locals (State :type "Array of /Game/MCTS/E_CellType Enum"))
  (bind _state (`local.State`))
  (for (_array_element _array_index) (`self.Cells`)
    (`KismetArrayLibrary.Array_Set` _state _array_index (`/Game/MCTS/BP_Cell.CurrentType` _array_element) true))
  (return _state))

(fn `MakeMove`
  (params (MoveSide :type "/Game/MCTS/E_CellType Enum" :default "NewEnumerator0") (Position :type Integer))
  (bind _currentstate (`self.GetCurrentState`))
  (bind _output (`|GetArrayItem` (`self.Cells`) Position))
  (bind _currenttype (`/Game/MCTS/BP_Cell.CurrentType` _output))
  (if (or (and (`|EnumEquality` _currenttype "NewEnumerator0") (`|EnumInequality` MoveSide "NewEnumerator0")) (`|EnumEquality` _currenttype MoveSide))
    (`/Game/MCTS/BP_Cell.SetType` _output MoveSide)
    (bind _wonside (`self.CheckWin` _currentstate))
    (if (or (`|EnumInequality` _wonside "NewEnumerator0") (== (`KismetArrayLibrary.Array_Find` _currentstate "NewEnumerator0") -1))
      (`self.ResetBoard`))
    (else
      (`KismetSystemLibrary.PrintString` "Illegal Move" true true (struct :`R` 1.0 :`A` 1.0)))))

(fn `ResetBoard`
  (for _array_element (`self.Cells`)
    (if (`|EnumInequality` (`/Game/MCTS/BP_Cell.CurrentType` _array_element) "NewEnumerator0")
      (`/Game/MCTS/BP_Cell.SetType` _array_element "NewEnumerator0")
      (`KismetSystemLibrary.PrintString` (`KismetStringLibrary.Concat_StrStr` (`KismetSystemLibrary.GetDisplayName` _array_element) " :: " (`|GetEnumeratorNameAsString` (`/Game/MCTS/BP_Cell.CurrentType` _array_element))))))
  (`KismetSystemLibrary.PrintString` "Reset"))

(fn `Start`
  (`self.EnableInput` (`GameplayStatics.GetPlayerController` 0))
  (`self.CreateCells`))

(fn `UserConstructionScript`)